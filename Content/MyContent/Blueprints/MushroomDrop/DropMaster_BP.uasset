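; DropMaster_BP is a mushroom drop point, apparently a base Blueprint, that awards points when a DLThirdPersonCharacter overlaps its Collision.
; The overlap passes DropType to the character's HasMushroom, then awards PointValue to player 0's character without branching on a result.
; In between, GetLife only gathers SphereOfInfluence's overlapping actors as PlantLife.
; A pickup type-matching check and a timer are left unconnected.
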(event OnComponentBeginOverlap(Collision)
  (params (OverlappedComponent :type Primitive%20Component%20Object%20Reference) (OtherActor :type Actor%20Object%20Reference) (OtherComp :type Primitive%20Component%20Object%20Reference) (OtherBodyIndex :type Integer) (bFromSweep :type Boolean) (SweepResult :type Hit%20Result%20Structure%20%28by%20ref%29))
  (bind _asdlthird_person_character (Utilities|Casting|CastToDLThirdPersonCharacter OtherActor))
  (Default|HasMushroom _asdlthird_person_character (Variables|Default|GetDropType))
  (CallFunction|GiveLifeWithinProxmity)
  (bind _asdlthird_person_character_2 (Utilities|Casting|CastToDLThirdPersonCharacter (Game|GetPlayerCharacter 0)))
  (Default|CallRecievePoints _asdlthird_person_character_2 (Variables|Default|GetPointValue)))

(event Custom|GiveLifeWithinProxmity
  (CallFunction|GetLife))

(event EventBeginPlay)

(event Collision|EventActorBeginOverlap
  (params (OtherActor :type Actor%20Object%20Reference)))

(event EventTick
  (params (DeltaSeconds :type Float%20%28single-precision%29)))

(fn ConstructionScript)

(fn GetLife
  (Variables|Default|SetPlantLife (Collision|GetOverlappingActors (Variables|Default|GetSphereOfInfluence) 0 :!class /Script/Engine.PrimitiveComponent)))