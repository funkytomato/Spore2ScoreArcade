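; DropZoneMaster_BP is a mushroom drop zone that accepts a mushroom of its DropType from the player character and boosts nearby life.
; On a Collision overlap with a matching carrier, it plays a cheer and sends a health boost to LifeMaster_BP actors inside SphereOfInfluence.
; It then awards points to player 0, reports the drop, resets their objective to collecting a mushroom, and expires shortly after.
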(event OnComponentBeginOverlap(Collision)
  (params (OverlappedComponent :type Primitive%20Component%20Object%20Reference) (OtherActor :type Actor%20Object%20Reference) (OtherComp :type Primitive%20Component%20Object%20Reference) (OtherBodyIndex :type Integer) (bFromSweep :type Boolean) (SweepResult :type Hit%20Result%20Structure%20%28by%20ref%29))
  (bind _asdlthird_person_character (Utilities|Casting|CastToDLThirdPersonCharacter OtherActor))
  (bind _isholding (Default|HasMushroom _asdlthird_person_character (Variables|Default|GetDropType)))
  (if _isholding
    (Audio|PlaySound2D "/Game/GameSoundCollection/Cartoon/Cue/Cartoon_ui_cheer_Cue.Cartoon_ui_cheer_Cue" 1.0 1.0 0.0 0 0)
    (CallFunction|GiveLifeWithinProxmity)
    (bind _asdlthird_person_character_2 (Utilities|Casting|CastToDLThirdPersonCharacter (Game|GetPlayerCharacter 0)))
    (Default|CallRecievePoints _asdlthird_person_character_2 (Variables|Default|GetPointValue))
    (Default|CallDroppedMushroom _asdlthird_person_character_2 (Variables|Default|GetDropType))
    (Variables|/Game/MyContent/Blueprints/Character/DynamicLocomotion/DLThirdPersonCharacter.DLThirdPersonCharacter_C|SetPlayerObjective _asdlthird_person_character_2 "Collect a Mushroom")
    (Actor|SetLifeSpan 2.0)
    (else
      (Development|PrintString "no mushroom"))))

(event Custom|GiveLifeWithinProxmity
  (bind _plantlife (Variables|Default|GetPlantLife))
  (CallFunction|GetLife)
  (Development|PrintString (Utilities|String|ToString(Integer) (Utilities|Array|Length _plantlife)))
  (Development|PrintString "LifeInProximity")
  (for _array_element _plantlife
    (bind _aslife_master_bp (Utilities|Casting|CastToLifeMaster_BP _array_element)
      (:then
        (Default|CallHealthBoost _aslife_master_bp (Variables|Default|GetHealthBoost))
        (Development|PrintString "Called DropZoneMaster health boost"))
      (:CastFailed
        (Development|PrintString "fail cast")))))

(event EventBeginPlay)

(event Collision|EventActorBeginOverlap
  (params (OtherActor :type Actor%20Object%20Reference)))

(event EventTick
  (params (DeltaSeconds :type Float%20%28single-precision%29)))

(fn ConstructionScript)

(fn GetLife
  (bind _sphereofinfluence (Variables|Default|GetSphereOfInfluence))
  (bind _overlappingactors (Collision|GetOverlappingActors _sphereofinfluence "/Game/MyContent/Environment/LifeMaster_BP.LifeMaster_BP_C" :!class /Script/Engine.PrimitiveComponent))
  (Variables|Default|SetPlantLife _overlappingactors)
  (Development|PrintString (Utilities|String|ToString(Integer) (Utilities|Array|Length _overlappingactors)))
  (Development|PrintString "Plant Life"))