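; Anim notify that spawns a footstep VFX at a bone on the animated mesh.
; Received_Notify casts the mesh owner to DLThirdPersonCharacter and takes the FootstepVFX system from that character, so the effect is defined per character rather than in the notify.
; It spawns unattached at the BoneName socket location plus a world-space offset, with the notify's rotation and scale, and returns false for any other owner.
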(fn ReceivedNotify
  (params (MeshComp :type Skeletal%20Mesh%20Component%20Object%20Reference) (Animation :type Anim%20Sequence%20Base%20Object%20Reference))
  (bind _returnvalue (Components|GetOwner MeshComp))
  (Utilities|IsValid _returnvalue
    (:Is%20Valid
      (bind _asdlthird_person_character (Utilities|Casting|CastToDLThirdPersonCharacter _returnvalue)
        (:then
          (Niagara|SpawnSystematLocation (Variables|/Game/MyContent/Blueprints/Character/DynamicLocomotion/DLThirdPersonCharacter.DLThirdPersonCharacter_C|GetFootstepVFX _asdlthird_person_character) (+ (Transformation|GetSocketLocation MeshComp (Variables|Default|GetBoneName)) (Variables|Default|GetLocationOffset)) (Variables|Default|GetRotationOffset) (Variables|Default|GetScaleOffset))
          (return true))
        (:CastFailed
          (return false))))
    (:Is%20Not%20Valid
      (return false))))