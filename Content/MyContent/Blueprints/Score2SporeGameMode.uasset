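; Game mode for Score2Spore that spawns the player's chosen character when play begins.
; On BeginPlay it loops over all PlayerStarts, storing each transform and the class from Score2SporeGameInstance's GetPlayerClass.
; A one-second Delay inside the loop collapses the iterations, so player controller 0's SpawnCharacter runs once, using the last start found.
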(event EventBeginPlay
  (bind _outactors (Actor|GetAllActorsOfClass "/Script/Engine.PlayerStart"))
  (for _array_element _outactors
    (Variables|Default|SetSpawnTransform (Transformation|GetActorTransform _array_element))
    (bind _asscore_2spore_game_instance (Utilities|Casting|CastToScore2SporeGameInstance (Game|GetGameInstance)))
    (bind _output_get (Variables|Default|SetGameInstanceRef _asscore_2spore_game_instance))
    (bind _class (Default|GetPlayerClass _output_get))
    (Variables|Default|SetClassToSpawn _class)
    (Utilities|FlowControl|Delay 1.0)
    (bind _asmy_player_controller_bp (Utilities|Casting|CastToMyPlayerController_BP (Game|GetPlayerController 0)))
    (Default|SpawnCharacter _asmy_player_controller_bp (Variables|Default|GetClassToSpawn) (Variables|Default|GetSpawnTransform))))

(event EventTick
  (params (DeltaSeconds :type Float%20%28single-precision%29)))

(fn ConstructionScript)