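; PlantGrowMaster_BP is a growable plant, apparently a master Blueprint, that changes its appearance as its health rises.
; Its LifeCycle override calls the parent, increases Health by GrowIncrementAmount, then checks which of three health bands up to 100 it falls in.
; Each band sets its stage mesh through a DoOnce that resets outside the band, so the mesh is only swapped on entering a new stage.
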(event EventBeginPlay
  (|CallParentFunction))

(event Collision|EventActorBeginOverlap
  (params (OtherActor :type Actor%20Object%20Reference))
  (|CallParentFunction OtherActor) ; This node is disabled and will not be called.\nDrag off pins to build functionality.
)

(event EventTick
  (params (DeltaSeconds :type Float%20%28single-precision%29))
  (|CallParentFunction DeltaSeconds) ; This node is disabled and will not be called.\nDrag off pins to build functionality.
)

(fn ConstructionScript
  (|CallParentFunction))

(fn LifeCycle
  (bind _health (Variables|Default|GetHealth))
  (bind _health_2 (Variables|Default|GetHealth))
  (bind _health_3 (Variables|Default|GetHealth))
  ;[1 1 1] Show Grow state on health
  (|CallParentFunction)
  (CallFunction|IncreaseHealth (Variables|Default|GetGrowIncrementAmount))
  (Utilities|FlowControl|Sequence
    (:then_0
      (if (and (> _health 0) (< _health 25))
        (Utilities|FlowControl|DoOnce false :!label _label
          (:Completed
            (Components|StaticMesh|SetStaticMesh (Variables|Default|GetStaticMesh) (Variables|Default|GetStage1))))
        (else
          (goto _label Reset))))
    (:then_1
      (if (and (> _health_2 24) (< _health_2 75))
        (Utilities|FlowControl|DoOnce false :!label _label_2
          (:Completed
            (Components|StaticMesh|SetStaticMesh (Variables|Default|GetStaticMesh) (Variables|Default|GetStage2))))
        (else
          (goto _label_2 Reset))))
    (:then_2
      (if (and (> _health_3 74) (< _health_3 101))
        (Utilities|FlowControl|DoOnce false :!label _label_3
          (:Completed
            (Components|StaticMesh|SetStaticMesh (Variables|Default|GetStaticMesh) (Variables|Default|GetStage3))))
        (else
          (goto _label_3 Reset))))))