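; BirchMaster_BP is an interactable birch tree Blueprint that extends a parent class's life cycle with a dead-tree appearance.
; Its LifeCycle override runs the parent logic, then checks IsDead.
; When dead, a DoOnce gate swaps the static mesh to DeadTreeMesh and assigns a branch material to the Branches slot.
; The event graph and construction script add no logic of their own.
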(event EventBeginPlay
  (|CallParentFunction) ; This node is disabled and will not be called.\nDrag off pins to build functionality.
)

(event Collision|EventActorBeginOverlap
  (params (OtherActor :type Actor%20Object%20Reference))
  (|CallParentFunction OtherActor) ; This node is disabled and will not be called.\nDrag off pins to build functionality.
)

(event EventTick
  (params (DeltaSeconds :type Float%20%28single-precision%29))
  (|CallParentFunction DeltaSeconds) ; This node is disabled and will not be called.\nDrag off pins to build functionality.
)

(fn ConstructionScript
  (|CallParentFunction))

(fn LifeCycle
  (bind _staticmesh (Variables|Default|GetStaticMesh))
  (|CallParentFunction)
  (if (Variables|Default|GetIsDead)
    (Utilities|FlowControl|DoOnce false
      (:Completed
        (Components|StaticMesh|SetStaticMesh _staticmesh (Variables|Default|GetDeadTreeMesh))
        (Rendering|Material|SetMaterialbyName _staticmesh "Branches" "/Game/PolygonNature/Materials/Mat_Tree_Branches_Inst.Mat_Tree_Branches_Inst")))))