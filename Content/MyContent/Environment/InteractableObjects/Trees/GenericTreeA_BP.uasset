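; Generic tree variant A, an interactable environment Blueprint that swaps to a dead-tree model when it dies.
; It overrides the inherited LifeCycle function, running the parent logic first, then checking IsDead.
; When dead, a DoOnce gate sets the static mesh to SM_Tree_Generic_Dead_01 a single time.
; The event graph holds only disabled default events, and the construction script just calls its parent.
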(event EventBeginPlay
  (|CallParentFunction) ; This node is disabled and will not be called.\nDrag off pins to build functionality.
)

(event Collision|EventActorBeginOverlap
  (params (OtherActor :type Actor%20Object%20Reference))
  (|CallParentFunction OtherActor) ; This node is disabled and will not be called.\nDrag off pins to build functionality.
)

(event EventTick
  (params (DeltaSeconds :type Float%20%28single-precision%29))
  (|CallParentFunction DeltaSeconds) ; This node is disabled and will not be called.\nDrag off pins to build functionality.
)

(fn ConstructionScript
  (|CallParentFunction))

(fn LifeCycle
  (|CallParentFunction)
  (if (Variables|Default|GetIsDead)
    (Utilities|FlowControl|DoOnce false
      (:Completed
        (Components|StaticMesh|SetStaticMesh (Variables|Default|GetStaticMesh) "/Game/PolygonNature/Meshes/Trees/SM_Tree_Generic_Dead_01.SM_Tree_Generic_Dead_01")))))