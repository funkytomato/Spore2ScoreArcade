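; Plant "Life" actor whose health drains while dying and rises on health boost events, with a brief decay pause at full health.
; A one-second looping LifeCycle timer applies decay, swaps leaf materials by health state and toggles a spotlight through paired DoOnce gates.
; Low health registers it on the Spawner's priority list; zero removes and destroys it.
; An overlap sphere shows its Life widget, turned toward the player's camera.
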(event OnComponentBeginOverlap(InteractionSphere)
  (params (OverlappedComponent :type Primitive%20Component%20Object%20Reference) (OtherActor :type Actor%20Object%20Reference) (OtherComp :type Primitive%20Component%20Object%20Reference) (OtherBodyIndex :type Integer) (bFromSweep :type Boolean) (SweepResult :type Hit%20Result%20Structure%20%28by%20ref%29))
  ;[1 1 1] Show Life Widget when nearby
  (Utilities|Casting|CastToDLThirdPersonCharacter OtherActor)
  (CallFunction|RotatetoFacePlayer)
  (Rendering|SetVisibility (Variables|Default|GetWidget) true false))

(event OnComponentEndOverlap(InteractionSphere)
  (params (OverlappedComponent :type Primitive%20Component%20Object%20Reference) (OtherActor :type Actor%20Object%20Reference) (OtherComp :type Primitive%20Component%20Object%20Reference) (OtherBodyIndex :type Integer))
  ;[1 1 1] Show Life Widget when nearby
  (Utilities|Casting|CastToDLThirdPersonCharacter OtherActor)
  (Rendering|SetVisibility (Variables|Default|GetWidget) false false))

(event Custom|RotateToFacePlayer
  ;[1 1 1] Rotate Widget to face Player
  (bind _asdlthird_person_character (Utilities|Casting|CastToDLThirdPersonCharacter (Game|GetPlayerCharacter 0)))
  (Transformation|SetWorldRotation (Variables|Default|GetWidget) (Math|Rotator|FindLookatRotation (Transformation|GetWorldLocation (Variables|Default|GetDefaultSceneRoot)) (Transformation|GetWorldLocation (Variables|/Game/MyContent/Blueprints/Character/DynamicLocomotion/DLThirdPersonCharacter.DLThirdPersonCharacter_C|GetFollowCamera _asdlthird_person_character))) false false))

(event Custom|DecreaseHealth
  (params (amount :type Integer))
  (bind _spawnerref (Variables|Default|GetSpawnerRef))
  ;[1 1 1] Increase/Decrease Health
  (bind _output_get (Variables|LifeStatus|SetHealth (Math|Integer|Clamp(Integer) (- (Variables|LifeStatus|GetHealth) amount) 0 100)))
  (if (< _output_get (Variables|LifeStatus|GetLowHealthValue))
    (if (== _output_get 0)
      (Default|CallRemoveLifefromScene _spawnerref self)
      (Default|CallRemoveLifefromPriority _spawnerref self)
      (Actor|DestroyActor)
      (else
        (Variables|LifeStatus|SetisLowHealth true)
        (Default|CallAddLifetoPriority (Variables|Default|GetSpawnerRef) self)))))

(event Custom|Illuminate
  ;[1 1 1] Illuminate/Unilluminate Life
  (Rendering|SetVisibility (Variables|Default|GetSpotLight) true false))

(event Custom|Unilluminate
  ;[1 1 1] Illuminate/Unilluminate Life
  (Rendering|SetVisibility (Variables|Default|GetSpotLight) false false))

(event Custom|HealthBoost_Event
  (params (amount :type Integer))
  ;[1 1 1] Set Timer and Assign Messages
  (CallFunction|IncreaseHealth amount))

(event Custom|IncreaseHealth
  (params (amount :type Integer))
  ;[1 1 1] Increase/Decrease Health
  (bind _output_get (Variables|LifeStatus|SetHealth (Math|Integer|Clamp(Integer) (+ (Variables|LifeStatus|GetHealth) amount) 0 100)))
  (if (>= _output_get (Variables|LifeStatus|GetLowHealthValue))
    (Variables|LifeStatus|SetisLowHealth false)
    (if (== _output_get 100)
      (Variables|LifeStatus|SetIsDying false)
      (Utilities|FlowControl|Delay 5.0)
      (Variables|LifeStatus|SetIsDying true))))

(event EventBeginPlay
  ;[1 1 1] Set Timer and Assign Messages
  (bind _returnvalue (Utilities|Time|SetTimerbyFunctionName 0 "LifeCycle" 1.0 true))
  (Variables|LifeStatus|SetLifeCycleTimer _returnvalue)
  (EventDispatchers|BindEventtoHealthBoost (delegate Custom|HealthBoost_Event))
  (bind _aslife_wbp (Utilities|Casting|CastToLife_WBP (UserInterface|GetUserWidgetObject (Variables|Default|GetWidget))))
  (Variables|/Game/MyContent/Widgets/Life_WBP.Life_WBP_C|SetOwner _aslife_wbp self)
  (bind _returnvalue_2 (Actor|GetActorOfClass "/Game/MyContent/Spawners/Spawner.Spawner_C"))
  (Variables|Default|SetSpawnerRef _returnvalue_2))

(fn ConstructionScript)

(fn LifeCycle
  (bind _self self)
  (bind _ishighhealth (Variables|LifeStatus|GetisHighHealth))
  (bind _returnvalue (Utilities|IsValid _self))
  (Utilities|FlowControl|Sequence
    (:then_0
      ;[1 1 1] Decrease the health of the plant
      (if (Variables|LifeStatus|GetIsDying)
        (CallFunction|DecreaseHealth 1)))
    (:then_1
      (if _returnvalue
        ;[1 1 1] Show respective material for health of plant
        (if (Variables|LifeStatus|GetisLowHealth)
          (Rendering|Material|SetMaterial (Variables|Default|GetStaticMesh) 0 (Variables|Visuals|GetBrownLeavesMaterial))
          (elif (not _ishighhealth)
            (Rendering|Material|SetMaterial (Variables|Default|GetStaticMesh) 0 (Variables|Visuals|GetGreenLeavesMaterial))
            (else
              (Rendering|Material|SetMaterial (Variables|Default|GetStaticMesh) 0 (Variables|Visuals|GetOldLeavesMaterial)))))))
    (:then_2
      (if _returnvalue
        ;[1 1 1] Illuminate plant if healthy
        (if _ishighhealth
          (Utilities|FlowControl|DoOnce false :!label _label
            (:Completed
              (CallFunction|Illuminate)
              (goto _label_2 Reset)))
          (else
            (Utilities|FlowControl|DoOnce false :!label _label_2
              (:Completed
                (CallFunction|Unilluminate)
                (goto _label Reset)))))))))