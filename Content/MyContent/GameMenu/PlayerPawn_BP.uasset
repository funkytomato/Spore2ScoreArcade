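; Menu pawn that shows the main menu on BeginPlay and handles the transition to character selection.
; GoToCharacterSelect removes the menu, moves the pawn toward the BusinessManInShirt transform on a timeline, then creates the selection widget without adding it to the viewport here.
; MoveLeft and MoveRight step a clamped three-slot index behind a CanClick gate that is never reset here; PlayerCharacterTimeline's switch has no actions.
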(event Custom|GoToCharacterSelect
  (Widget|RemovefromParent (Variables|Default|GetMainMenuWidget))
  (bind _alpha (Timeline|CharacterSelect PlayFromStart)
    (:Update
      (Transformation|SetActorTransform (Math|Transform|Lerp(Transform) (Transformation|GetActorTransform) (Variables|Default|GetBusinessManInShirtTransform) _alpha)))
    (:Finished
      (UserInterface|CreateWidget "/Game/MyContent/GameMenu/CharacterSelectionMenu_BP.CharacterSelectionMenu_BP_C" 0 0))))

(event Custom|MoveRight
  (if (and (< (Variables|Default|GetArrowCount) 2) (Variables|Default|GetCanClick?))
    (Variables|Default|SetCanClick? false)
    (Variables|Default|SetArrowCount (Math|Integer|Clamp(Integer) (+ (Variables|Default|GetArrowCount) 1) 0 2))))

(event Custom|MoveLeft
  (if (and (> (Variables|Default|GetArrowCount) 0) (Variables|Default|GetCanClick?))
    (Variables|Default|SetCanClick? false)
    (Variables|Default|SetArrowCount (Math|Integer|Clamp(Integer) (- (Variables|Default|GetArrowCount) 1) 0 2))))

(event Custom|PlayerCharacterTimeline
  (params (Arrow :type Integer))
  (switch int Arrow))

(event EventBeginPlay
  (bind _returnvalue (UserInterface|CreateWidget "/Game/MyContent/GameMenu/MainMenuWidget_BP.MainMenuWidget_BP_C"))
  (bind _output_get (Variables|Default|SetMainMenuWidget _returnvalue))
  (UserInterface|Viewport|AddtoViewport _output_get 0))

(fn ConstructionScript)